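; Player controller for an auto-chess game, handling the hover info panel, deck config, card purchases and match-end screen.
; BeginPlay maps chess classes to skill descriptions from DT_CHess.
; Tick traces pawns under the cursor, showing a WBP_Chess built from the piece's data row and fading it via timeline when hover leaves.
; Events forward card purchases, destroy selected actors, set the deck, and swap the main window for WBP_EndGame.
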(event Custom|SetWidget
  (params (MainWindow :type WBP%20Main%20Window%20Object%20Reference))
  (Variables|Default|SetMain%20Window MainWindow))

(event Custom|DestroySelectedActor
  (params (ActorRef :type Actor%20Object%20Reference))
  (Actor|DestroyActor ActorRef))

(event Custom|SetDeck
  (params (TargetArray :type Array%20of%20Auto%20Chess%20Card%20Base%20Class%20References) (Isini? :type Boolean))
  (if Isini?
    (Utilities|Array|Clear (Variables|Default|GetDeckConfig)))
  (Utilities|Array|AppendArray (Variables|Default|GetDeckConfig) TargetArray))

(event Custom|ServerBuyCard
  (params (CardClass :type Auto%20Chess%20Card%20Base%20Class%20Reference))
  (Class|AutoChessPlayerController|BuyCard CardClass))

(event EventBeginPlay
  (bind _outrownames (DataTable|GetDataTableRowNames "/Game/Blueprints/Units/Chess/DA/DT_CHess.DT_CHess"))
  (for _array_element _outrownames
    (bind _returnvalue (Utilities|GetDataTableRow "/Game/Blueprints/Units/Chess/DA/DT_CHess.DT_CHess" _array_element)
      (:then
        (Utilities|Map|Add (Variables|Default|GetNewVar) (.Class (Utilities|Struct|BreakST_ChessData _returnvalue)) (.SkillDesc (Utilities|Struct|BreakST_ChessData _returnvalue)))))))

(event EventOnMatchEnded
  (params (WinnerTeamID :type Integer))
  (bind _returnvalue (UserInterface|CreateWidget "/Game/buildsystem/UI/EndGame/WBP_EndGame.WBP_EndGame_C" self WinnerTeamID))
  (UserInterface|Viewport|AddtoViewport _returnvalue 0)
  (Widget|SetVisibility (Variables|Default|GetMain%20Window) "Hidden"))

(event EventTick
  (params (DeltaSeconds :type Float%20%28single-precision%29))
  (bind _array (Utilities|Array|MakeArray "ObjectTypeQuery3"))
  (bind _main_window (Variables|Default|GetMain%20Window))
  (bind _hitresult (Class|PlayerController|GetHitResultUnderCursorforObjects _array true))
  (bind _forchess (Variables|/Game/buildsystem/UI/WBP_MainWindow.WBP_MainWindow_C|GetForChess _main_window))
  (bind _hitactor (Collision|BreakHitResult _hitresult))
  (if (not (== _hitactor (Variables|Default|GetHit%20Actor)))
    (bind _output_get (Variables|Default|SetHit%20Actor _hitactor))
    (bind _asbp_chessman_master (Utilities|Casting|CastToBP_ChessmanMaster _output_get)
      (:then
        (bind _returnvalue (UserInterface|CreateWidget "/Game/buildsystem/UI/Preparation/WBP_Chess.WBP_Chess_C" 0 "" (CallFunction|GetChessRow _asbp_chessman_master)))
        (Variables|Default|SetNewVar_0 _returnvalue)
        (Widget|Panel|ClearChildren _forchess)
        (Widget|Panel|AddChild _forchess (Variables|Default|GetNewVar_0)))
      (:CastFailed
        (bind _新建轨道_0 (Timeline|时间轴 PlayFromStart)
          (:Update
            (Utilities|IsValid (Variables|Default|GetNewVar_0)
              (:Is%20Valid
                (Widget|SetRenderOpacity (Variables|Default|GetNewVar_0) _新建轨道_0))))
          (:Finished
            (Widget|Panel|ClearChildren (Variables|/Game/buildsystem/UI/WBP_MainWindow.WBP_MainWindow_C|GetForChess (Variables|Default|GetMain%20Window)))
            (Utilities|IsValid (Variables|Default|GetNewVar_0)
              (:Is%20Valid
                (Widget|SetRenderOpacity (Variables|Default|GetNewVar_0) 1.0)))))))))

(fn ConstructionScript)

(fn ServerDeleteActor)

(fn GetChessRow
  (params (Target :type Auto%20Chess%20Unit%20Base%20Object%20Reference))
  (bind _unitdatahandle (Variables|/Script/AutoChess.AutoChessUnitBase|GetUnitDataHandle Target))
  (bind (_datatable _rowname) (Utilities|Struct|BreakDataTableRowHandle _unitdatahandle))
  (bind _returnvalue (Utilities|GetDataTableRow _datatable _rowname)
    (:then
      (return _returnvalue))))