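; Auto chess game state that serves as a lookup for buff textures by gameplay tag.
; On BeginPlay it reads every row of DT_Buffinfo and caches each tag and texture pair in the BuffAppear map.
; GetBuffTexture returns the cached texture for a given tag, while ChessClicked is an empty stub.
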(event EventBeginPlay
  (bind _outrownames (DataTable|GetDataTableRowNames "/Game/buildsystem/UI/HpBar/DT_Buffinfo.DT_Buffinfo"))
  (for _array_element _outrownames
    (bind _returnvalue (Utilities|GetDataTableRow "/Game/buildsystem/UI/HpBar/DT_Buffinfo.DT_Buffinfo" _array_element)
      (:then
        (Utilities|Map|Add (Variables|Default|GetBuffAppear) (.GameplayTag (Utilities|Struct|BreakST_BuffInfo _returnvalue)) (.Texture (Utilities|Struct|BreakST_BuffInfo _returnvalue))))))
  (Variables|Default|SetNewVar (Utilities|Map|Length (Variables|Default|GetBuffAppear)))
  (if true
    _))

(fn ConstructionScript)

(fn ChessClicked
  (return 0))

(fn GetBuffTexture
  (params (GETag :type Gameplay%20Tag%20Structure))
  (return (.Value (Utilities|Map|Find (Variables|Default|GetBuffAppear) GETag))))