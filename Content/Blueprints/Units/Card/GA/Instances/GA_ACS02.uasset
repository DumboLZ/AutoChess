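; GA_ACS02 is an event-activated Gameplay Ability for card units that grants Valor to queried targets.
; It applies five stacks of GE_ValorBase to each target data entry from TargetQuery.
; After a short delay it sends the Valor special gameplay event to the target actors, directly with authority or through the ACS02Rpc custom event otherwise.
; Short delays precede EndAbility, both inside the target loop and after it.
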(event Custom|ACS02Rpc
  (Ability|SendGameplayEventtoActor (stale Ability|EventActivateAbilityFromEvent _array_element_2) "(TagName=\"AutoChess.Event.Specials.Valor\")"))

(event Ability|EventActivateAbilityFromEvent
  (params (EventData :type Gameplay%20Event%20Data%20Structure%20%28by%20ref%29))
  (bind _newlocalvar1 (CallFunction|TargetQuery EventData))
  (for _array_element _newlocalvar1
    (Utilities|FlowControl|Sequence
      (:then_0
        (GameplayEffects|ApplyGameplayEffectToTarget _array_element "/Game/Blueprints/Units/Chess/GE/GE_ValorBase.GE_ValorBase_C" 1 5))
      (:then_1
        (Utilities|FlowControl|Delay 0.1)
        (for _array_element_2 (Ability|TargetData|GetAllActorsfromTargetData _array_element)
          (Ability|HasAuthority
            (:True
              (Ability|SendGameplayEventtoActor _array_element_2 "(TagName=\"AutoChess.Event.Specials.Valor\")"))
            (:False
              (CallFunction|ACS02Rpc)))))
      (:then_2
        (Utilities|FlowControl|Delay 0.2)
        (Ability|EndAbility))))
  (Utilities|FlowControl|Delay 0.2)
  (Ability|EndAbility))

(fn ServerRPC)