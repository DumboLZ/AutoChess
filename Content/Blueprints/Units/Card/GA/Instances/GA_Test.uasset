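; Test card gameplay ability that converts the instigating player's mana into shield for queried targets in the auto-chess game.
; On activation from an event, it casts the instigator to the player controller and runs a target query on the event data.
; Each target receives GE_Shield with stacks scaled by whole mana points, leaving only the fractional mana.
; The ability ends only on the positive-mana path.
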(event Ability|EventActivateAbilityFromEvent
  (params (EventData :type Gameplay%20Event%20Data%20Structure%20%28by%20ref%29))
  (bind _asauto_chess_player_controller (Utilities|Casting|CastToAutoChessPlayerController (.Instigator (Utilities|Struct|BreakGameplayEventData EventData))))
  (if (> (Variables|/Script/AutoChess.AutoChessPlayerController|GetMana _asauto_chess_player_controller) 0.0)
    (bind _newlocalvar1 (CallFunction|TargetQuery EventData))
    (for _array_element _newlocalvar1
      (GameplayEffects|ApplyGameplayEffectToTarget _array_element "/Game/Blueprints/Units/Card/GE/GE_Shield.GE_Shield_C" 1 (* (.ReturnValue (Math|Float|Division(WholeandRemainder) (Variables|/Script/AutoChess.AutoChessPlayerController|GetMana _asauto_chess_player_controller) 1.0)) 15)))
    (Variables|/Script/AutoChess.AutoChessPlayerController|SetMana _asauto_chess_player_controller (.Remainder (Math|Float|Division(WholeandRemainder) (Variables|/Script/AutoChess.AutoChessPlayerController|GetMana _asauto_chess_player_controller) 1.0)))
    (Ability|EndAbility)))