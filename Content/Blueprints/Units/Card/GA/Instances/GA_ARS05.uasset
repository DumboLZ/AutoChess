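; GA_ARS05 is an event-triggered auto-chess unit ability that grants Valor to queried targets in repeated passes.
; It runs TargetQuery once, then applies GE_ValorBase stacks to each target and sends a Valor special event to its actors.
; Next-tick delays separate effect, event and pass, and a counter ends the ability after three passes over the same targets.
; An older owner-only Valor chain remains unconnected.
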(event Ability|EventActivateAbility)

(event Ability|EventOnEndAbility
  (params (bWasCancelled :type Boolean)))

(event EventActivateAbilityfromEvent
  (params (EventData :type Gameplay%20Event%20Data%20Structure%20%28by%20ref%29))
  (Variables|Default|Set122 0)
  (bind _newlocalvar1 (CallFunction|TargetQuery EventData))
  (Variables|Default|SetNew%20Local%20Var%201 _newlocalvar1)
  (for _array_element (Variables|Default|GetNew%20Local%20Var%201) :!label _label
    (GameplayEffects|ApplyGameplayEffectToTarget _array_element "/Game/Blueprints/Units/Chess/GE/GE_ValorBase.GE_ValorBase_C" 1 3)
    (Utilities|FlowControl|DelayUntilNextTick)
    (for _array_element_2 (Ability|TargetData|GetAllActorsfromTargetData _array_element)
      (Ability|SendGameplayEventtoActor _array_element_2 "(TagName=\"AutoChess.Event.Specials.Valor\")")))
  (Utilities|FlowControl|DelayUntilNextTick)
  (bind _result (Math|Integer|IncrementInt (Variables|Default|Get122))
    (:%20%20
      (if (>= _result 3)
        (Ability|EndAbility)
        (else
          (goto _label))))))