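; GA_GUS01 is an auto-chess card ability that damages and stuns units across a set of grid cells, apparently a 3x3 area.
; Event activation waits briefly, then reads the cells from the payload via Get33FromPayload and looks up each unit through AutoChessGameState.
; Each unit receives stacked GE_Damage_Normal and GE_Stunned effects.
; The graph never calls EndAbility, and its 40HP comments do not match the stack counts.
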(event Ability|EventActivateAbility)

(event Ability|EventOnEndAbility
  (params (bWasCancelled :type Boolean)))

(event Ability|EventActivateAbilityFromEvent
  (params (EventData :type Gameplay%20Event%20Data%20Structure%20%28by%20ref%29))
  (Utilities|FlowControl|Delay 1.0)
  (for _array_element (CallFunction|Get3*3fromPayload EventData)
    (bind _returnvalue (Class|AutoChessGameState|GetUnitatGrid (.AsAuto%20Chess%20Game%20State (Utilities|Casting|CastToAutoChessGameState (Game|GetGameState))) (.X (Utilities|Struct|BreakIntPoint _array_element)) (.Y (Utilities|Struct|BreakIntPoint _array_element))))
    (GameplayEffects|ApplyGameplayEffectToTarget (Ability|TargetData|AbilityTargetDatafromActor _returnvalue) "/Game/Blueprints/Units/Card/GE/GE_Damage_Normal.GE_Damage_Normal_C" 1 100) ; 流失40HP
    (GameplayEffects|ApplyGameplayEffectToTarget (Ability|TargetData|AbilityTargetDatafromActor _returnvalue) "/Game/Blueprints/Units/Chess/GE/GE_Stunned.GE_Stunned_C" 1 3) ; 流失40HP
  ))