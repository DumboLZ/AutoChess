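; Gameplay ability for the Fireball card in an auto-chess game, triggered by a gameplay event to damage a unit.
; 查询目标 (query target) scans the source card's highlighted tiles and filters units by the card's TargetType against the instigating player's TeamID.
; It returns only the first matching unit, which receives GE_FireballDamage before the ability ends.
; An AOE radius query is left unconnected.
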(event Ability|EventActivateAbilityFromEvent
  (params (EventData :type Gameplay%20Event%20Data%20Structure%20%28by%20ref%29))
  (bind _returnvalue (|查询目标 EventData))
  (GameplayEffects|ApplyGameplayEffectToTarget _returnvalue "/Game/Blueprints/Units/Card/GE/GE_FireballDamage.GE_FireballDamage_C" 1 1)
  (Ability|EndAbility))