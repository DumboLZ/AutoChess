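; Gameplay ability for card unit AUS02 of Clan A, triggered by a gameplay event, that applies a stacked effect based on target state.
; It runs a target query on the event data and checks an attribute on each resulting actor's ability system.
; A positive attribute selects a higher stack count than the fallback, but only the fallback call passes the target data.
; The ability ends once all targets are processed.
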(event Ability|EventActivateAbilityFromEvent
  (params (EventData :type Gameplay%20Event%20Data%20Structure%20%28by%20ref%29))
  (bind _newlocalvar1 (CallFunction|TargetQuery EventData))
  (for _array_element _newlocalvar1
    (for _array_element_2 (Ability|TargetData|GetActorsfromTargetData _array_element)
      (if (and (.bSuccessfullyFoundAttribute (Ability|Attribute|GetFloatAttributefromAbilitySystemComponent (Ability|GetAbilitySystemComponent _array_element_2) "(AttributeName=\"Shield\",Attribute=/Script/AutoChess.AutoChessAttributeSet:Shield,AttributeOwner=\"/Script/CoreUObject.Class'/Script/AutoChess.AutoChessAttributeSet'\")")) (> (.ReturnValue (Ability|Attribute|GetFloatAttributefromAbilitySystemComponent (Ability|GetAbilitySystemComponent _array_element_2) "(AttributeName=\"Shield\",Attribute=/Script/AutoChess.AutoChessAttributeSet:Shield,AttributeOwner=\"/Script/CoreUObject.Class'/Script/AutoChess.AutoChessAttributeSet'\")")) 0.0))
        (GameplayEffects|ApplyGameplayEffectToTarget :Stacks 225)
        (else
          (GameplayEffects|ApplyGameplayEffectToTarget _array_element 0 1 150)))))
  (Ability|EndAbility))