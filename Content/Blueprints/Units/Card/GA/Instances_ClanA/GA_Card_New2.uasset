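; GA_Card_New2 is a card gameplay ability in an auto-chess game that launches baseball projectiles at queried targets.
; When activated by an event, it runs a target query and spawns a side-offset BP_BaseBall at every actor found, using the instigating player's team ID.
; Each projectile carries fixed damage and applies GE_Card_New2 to both enemies and friendlies.
; The ability ends after a short delay.
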(event Ability|EventActivateAbilityFromEvent
  (params (EventData :type Gameplay%20Event%20Data%20Structure%20%28by%20ref%29))
  (bind _array (Utilities|Array|MakeArray (Utilities|Struct|MakeProjectileEffectInfo "/Game/Blueprints/Units/Card/GE/GE_Card_New2.GE_Card_New2_C" 1.0)))
  (bind _newlocalvar1 (CallFunction|TargetQuery EventData))
  (for _array_element _newlocalvar1
    (for _array_element_2 (Ability|TargetData|GetActorsfromTargetData _array_element)
      (Class|AutoChessCardBase|SpawnProjectilefromSide _array_element_2 "/Game/Blueprints/Units/BP_BaseBall.BP_BaseBall_C" 4e+01 (Variables|/Script/AutoChess.AutoChessPlayerController|GetTeamID (.AsAuto%20Chess%20Player%20Controller (Utilities|Casting|CastToAutoChessPlayerController (.Instigator (Utilities|Struct|BreakGameplayEventData EventData))))) _array _array 3e+02)))
  (Utilities|FlowControl|Delay 0.5)
  (Ability|EndAbility))