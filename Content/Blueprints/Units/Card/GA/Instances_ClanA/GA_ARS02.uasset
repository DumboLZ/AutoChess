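; GA_ARS02 is a Clan A card gameplay ability that converts the instigating player controller's mana into damage.
; When mana is positive, it spends all whole points, scales damage by that count and keeps the fractional remainder.
; Each TargetQuery result receives GE_Damage_Normal, with the damage passed as stack count, boosted by half if an attribute on the event target is positive.
; EndAbility is only reached inside the positive-mana branch.
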(event Ability|EventActivateAbilityFromEvent
  (params (EventData :type Gameplay%20Event%20Data%20Structure%20%28by%20ref%29))
  (bind (_eventtag _instigator _target) (Utilities|Struct|BreakGameplayEventData EventData))
  (bind _returnvalue (Ability|GetAbilitySystemComponent _target))
  (bind (_bsuccessfullyfoundattribute _returnvalue_2) (Ability|Attribute|GetFloatAttributefromAbilitySystemComponent _returnvalue "(AttributeName=\"Shield\",Attribute=/Script/AutoChess.AutoChessAttributeSet:Shield,AttributeOwner=\"/Script/CoreUObject.Class'/Script/AutoChess.AutoChessAttributeSet'\")"))
  (bind _asauto_chess_player_controller (Utilities|Casting|CastToAutoChessPlayerController _instigator))
  (if (> (Variables|/Script/AutoChess.AutoChessPlayerController|GetMana _asauto_chess_player_controller) 0.0)
    (Variables|Default|SetCacheDamage (* (.ReturnValue (Math|Float|Division(WholeandRemainder) (Variables|/Script/AutoChess.AutoChessPlayerController|GetMana _asauto_chess_player_controller) 1.0)) 20))
    (bind _newlocalvar1 (CallFunction|TargetQuery EventData))
    (for _array_element _newlocalvar1
      (GameplayEffects|ApplyGameplayEffectToTarget _array_element "/Game/Blueprints/Units/Card/GE/GE_Damage_Normal.GE_Damage_Normal_C" 1 (Math|Integer|SelectInt (Math|Float|Truncate (* (Variables|Default|GetCacheDamage) 1.5)) (Variables|Default|GetCacheDamage) (and _bsuccessfullyfoundattribute (> _returnvalue_2 0.0)))))
    (Variables|/Script/AutoChess.AutoChessPlayerController|SetMana _asauto_chess_player_controller (.Remainder (Math|Float|Division(WholeandRemainder) (Variables|/Script/AutoChess.AutoChessPlayerController|GetMana _asauto_chess_player_controller) 1.0)))
    (Ability|EndAbility)))