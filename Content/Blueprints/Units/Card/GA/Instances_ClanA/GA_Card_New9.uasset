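; GA_Card_New9 is a Clan A card gameplay ability that casts random cards on its targets in the auto chess game.
; On event activation, it runs a target query and takes the actors from each target data result.
; Each actor receives three cards drawn from an equally weighted pool of seven ANCCS cards, using the instigating player controller's team ID.
; The ability ends after a short delay.
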(event Ability|EventActivateAbilityFromEvent
  (params (EventData :type Gameplay%20Event%20Data%20Structure%20%28by%20ref%29))
  (bind _newlocalvar1 (CallFunction|TargetQuery EventData))
  (for _array_element _newlocalvar1
    (for _array_element_2 (Ability|TargetData|GetActorsfromTargetData _array_element)
      (Class|AutoChessCardBase|CastRandomCardsonTarget _array_element_2 3 (Utilities|Array|MakeArray (Utilities|Struct|MakeWeightedCardEntry "/Game/Blueprints/Units/Card/Instance/Cards_NewAlpha/BP_ANCCS01.BP_ANCCS01_C" 1.0) (Utilities|Struct|MakeWeightedCardEntry "/Game/Blueprints/Units/Card/Instance/Cards_NewAlpha/BP_ANCCS02.BP_ANCCS02_C" 1.0) (Utilities|Struct|MakeWeightedCardEntry "/Game/Blueprints/Units/Card/Instance/Cards_NewAlpha/BP_ANCCS03.BP_ANCCS03_C" 1.0) (Utilities|Struct|MakeWeightedCardEntry "/Game/Blueprints/Units/Card/Instance/Cards_NewAlpha/BP_ANCCS04.BP_ANCCS04_C" 1.0) (Utilities|Struct|MakeWeightedCardEntry "/Game/Blueprints/Units/Card/Instance/Cards_NewAlpha/BP_ANCCS05.BP_ANCCS05_C" 1.0) (Utilities|Struct|MakeWeightedCardEntry "/Game/Blueprints/Units/Card/Instance/Cards_NewAlpha/BP_ANCCS06.BP_ANCCS06_C" 1.0) (Utilities|Struct|MakeWeightedCardEntry "/Game/Blueprints/Units/Card/Instance/Cards_NewAlpha/BP_ANCCS07.BP_ANCCS07_C" 1.0)) (Variables|/Script/AutoChess.AutoChessPlayerController|GetTeamID (.AsAuto%20Chess%20Player%20Controller (Utilities|Casting|CastToAutoChessPlayerController (.Instigator (Utilities|Struct|BreakGameplayEventData EventData))))))))
  (Utilities|FlowControl|Delay 0.5)
  (Ability|EndAbility))