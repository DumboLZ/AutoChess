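; Auto-chess unit Blueprint in the NewFlameSoul set that shows its team and skill readiness visually.
; On BeginPlay it tags itself with its TeamID and builds a dynamic icon material on its Plane from its data table row, tinted by team.
; A looping timer polls an ability system attribute against a threshold, and on each readiness change timelines scale the Cube up or back down.
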(event Custom|CustomEvent
  (bind _abilitysystemcomponent (Variables|Default|GetAbilitySystemComponent))
  (bind _cube (Variables|Default|GetCube))
  (bind _returnvalue (Ability|Attribute|GetFloatAttributefromAbilitySystemComponent _abilitysystemcomponent "(AttributeName=\"Mana\",Attribute=/Script/AutoChess.AutoChessAttributeSet:Mana,AttributeOwner=\"/Script/CoreUObject.Class'/Script/AutoChess.AutoChessAttributeSet'\")"))
  (bind _returnvalue_2 (> _returnvalue 95.0))
  (if (== (Variables|Default|GetIsSkillReady) _returnvalue_2)
    (Utilities|FlowControl|DoOnce false :!label _label
      (:Completed
        (if (Variables|Default|GetIsSkillReady)
          (bind _newtrack_0 (Timeline|Timeline PlayFromStart)
            (:Update
              (Transformation|SetRelativeScale3D _cube (Math|Vector|Lerp(Vector) (Variables|/Script/Engine.SceneComponent|GetRelativeScale3D (Variables|Default|GetCube)) (* (Variables|Default|GetFirstScale) "1.500000,1.500000,1.500000") _newtrack_0))))
          (else
            (bind _newtrack_0_2 (Timeline|Timeline_0 PlayFromStart)
              (:Update
                (Transformation|SetRelativeScale3D _cube (Math|Vector|Lerp(Vector) (Variables|/Script/Engine.SceneComponent|GetRelativeScale3D (Variables|Default|GetCube)) (Variables|Default|GetFirstScale) _newtrack_0_2))))))))
    (else
      (Variables|Default|SetIsSkillReady _returnvalue_2)
      (goto _label Reset))))

(event EventBeginPlay
  (bind _tags (Variables|Default|GetTags))
  (bind _unitdatahandle (Variables|Default|GetUnitDataHandle))
  (bind (_datatable _rowname) (Utilities|Struct|BreakDataTableRowHandle _unitdatahandle))
  (Utilities|FlowControl|Delay 0.2)
  (Utilities|Array|Clear _tags)
  (Utilities|Array|AddUnique _tags (Utilities|String|StringToName (Utilities|String|ToString(Integer) (Variables|Default|GetTeamID))))
  (Variables|Default|SetFirstScale (Variables|/Script/Engine.SceneComponent|GetRelativeScale3D (Variables|Default|GetCube)))
  (Utilities|Time|SetTimerbyEvent (delegate Custom|CustomEvent) 0.2 true)
  (bind _returnvalue (Utilities|GetDataTableRow _datatable _rowname)
    (:then
      (bind _returnvalue_2 (Rendering|Material|CreateDynamicMaterialInstance (Variables|Default|GetPlane) 0 "/Game/Art/M_UnitIcon_Inst.M_UnitIcon_Inst" "None" :!class /Script/Engine.PrimitiveComponent))
      (Variables|Default|SetMaterial _returnvalue_2)
      (Rendering|Material|SetTextureParameterValue (Variables|Default|GetMaterial) "Icon" (.Icon (Utilities|Struct|BreakAutoChessUnitRow _returnvalue)))
      (Rendering|Material|SetVectorParameterValue (Variables|Default|GetMaterial) "Tint" (Utilities|Select :Index (Variables|Default|GetTeamID) :Option%200 "(R=0.169710,G=0.781250,B=0.000000,A=1.000000)" :Option%201 "(R=0.307292,G=0.076449,B=0.070334,A=1.000000)") :!class /Script/Engine.MaterialInstanceDynamic)
      (Rendering|Material|SetMaterial (Variables|Default|GetPlane) 0 (Variables|Default|GetMaterial))
      (Transformation|AddWorldRotation (Variables|Default|GetPlane) "0.000000,90.000000,0.000000" false false))))

(fn ConstructionScript)

(fn ChessClicked
  (return 0))

(fn GetBuffTexture
  (params (GETag :type Gameplay%20Tag%20Structure))
  (return 0))