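; GA_ANSC03 is a gameplay ability for an auto-chess unit that fires a baseball projectile at the nearest opposing unit.
; On activation it gets the opposing team's units from the game state and loops over them to keep the closest to the owner.
; The owning chessman spawns the BP_BaseBall projectile at that target with fixed damage.
; The ability ends only after firing; without a valid target, EndAbility is never called.
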(event Ability|EventActivateAbility
  (bind _returnvalue (Class|GameplayAbility|MakeTargetLocationInfofromOwnerActor))
  (bind _sourceactor (Utilities|Struct|BreakGameplayAbilityTargetingLocationInfo _returnvalue))
  (bind _asbp_chessman_master (Utilities|Casting|CastToBP_ChessmanMaster _sourceactor))
  (bind _asbp_auto_chess_game_state (Utilities|Casting|CastToBP_AutoChessGameState (Game|GetGameState)))
  (bind _returnvalue_2 (Class|AutoChessGameState|GetUnitsbyTeam _asbp_auto_chess_game_state (Math|Integer|Absolute(Integer) (- (Variables|/Script/AutoChess.AutoChessUnitBase|GetTeamID _asbp_chessman_master) 1))))
  (for _array_element _returnvalue_2
    (if (!= _array_element _sourceactor)
      (if (< (Transformation|GetDistanceTo _array_element _sourceactor) (Variables|Default|GetNewVar_0))
        (Variables|Default|SetNewVar_0 (Transformation|GetDistanceTo _array_element _sourceactor))
        (Variables|Default|SetArray%20Element _array_element))))
  (Utilities|IsValid (Variables|Default|GetArray%20Element)
    (:Is%20Valid
      (Class|AutoChessUnitBase|SpawnProjectileatTarget _asbp_chessman_master (Variables|Default|GetArray%20Element) "/Game/Blueprints/Units/BP_BaseBall.BP_BaseBall_C" 4e+01 false)
      (Ability|EndAbility))))