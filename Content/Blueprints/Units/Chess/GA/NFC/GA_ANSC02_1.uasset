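; Gameplay ability for an auto chess unit (ANSC02) that deals area attack damage to non-allied units around its owner.
; On activation it takes the cells from GetGrid33 at the owner's current grid position and looks up each cell's unit through the game state.
; Units with a different TeamID receive GE_DealAttackDamage.
; The graph makes no EndAbility call and has no explicit empty-cell check.
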(event Ability|EventActivateAbility
  (bind _asauto_chess_unit_base (Utilities|Casting|CastToAutoChessUnitBase (.SourceActor (Utilities|Struct|BreakGameplayAbilityTargetingLocationInfo (Class|GameplayAbility|MakeTargetLocationInfofromOwnerActor)))))
  (Variables|Default|SetTeam%20ID (Variables|/Script/AutoChess.AutoChessUnitBase|GetTeamID _asauto_chess_unit_base))
  (bind _outputpoints (CallFunction|GetGrid3*3 (Variables|/Script/AutoChess.AutoChessUnitBase|GetCurrentGridPos _asauto_chess_unit_base)))
  (for _array_element _outputpoints
    (bind _asauto_chess_game_state (Utilities|Casting|CastToAutoChessGameState (Game|GetGameState)))
    (bind _returnvalue (Class|AutoChessGameState|GetUnitatGrid _asauto_chess_game_state (.X (Utilities|Struct|BreakIntPoint _array_element)) (.Y (Utilities|Struct|BreakIntPoint _array_element))))
    (if (not (== (Variables|/Script/AutoChess.AutoChessUnitBase|GetTeamID _returnvalue) (Variables|Default|GetTeam%20ID)))
      (GameplayEffects|ApplyGameplayEffectToTarget (Ability|TargetData|AbilityTargetDatafromActor _returnvalue) "/Game/Blueprints/Units/Chess/GE/GE_DealAttackDamage.GE_DealAttackDamage_C" 1 1) ; 造成攻击力伤害
    )))

(event Ability|EventOnEndAbility
  (params (bWasCancelled :type Boolean)))