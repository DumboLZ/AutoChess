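; GA_ANSC05 is an auto-chess unit Gameplay Ability that grants mana to the owner's allied BurnSoul Thrower units.
; On activation it gets every unit on the owner's TeamID from the game state and checks each ability system for the Clan.BurnSoul.Chess.Thrower tag.
; Each match receives GE_AddMana1 at a high stack count to scale the gain, then the ability ends immediately.
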(event Ability|EventActivateAbility
  (bind _asbp_auto_chess_game_state (Utilities|Casting|CastToBP_AutoChessGameState (Game|GetGameState)))
  (bind _returnvalue (Class|AutoChessGameState|GetUnitsbyTeam _asbp_auto_chess_game_state (Variables|/Script/AutoChess.AutoChessUnitBase|GetTeamID (.AsAuto%20Chess%20Unit%20Base (Utilities|Casting|CastToAutoChessUnitBase (.SourceActor (Utilities|Struct|BreakGameplayAbilityTargetingLocationInfo (Class|GameplayAbility|MakeTargetLocationInfofromOwnerActor))))))))
  (for _array_element _returnvalue
    (bind _returnvalue_2 (GameplayTags|HasAnyMatchingGameplayTags(Message) (Ability|GetAbilitySystemComponent _array_element) (GameplayTags|MakeLiteralGameplayTagContainer "(GameplayTags=((TagName=\"Clan.BurnSoul.Chess.Thrower\")))")))
    (if _returnvalue_2
      (GameplayEffects|ApplyGameplayEffectToTarget (Ability|TargetData|AbilityTargetDatafromActor _array_element) "/Game/Blueprints/Units/Card/GE/GE_AddMana1.GE_AddMana1_C" 1 100)))
  (Ability|EndAbility))