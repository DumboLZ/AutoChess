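; GA_ANSCS01_A is a gameplay ability for an auto-chess unit that grants Valor to its team.
; On activation it applies a stacked periodic mana effect to its owner and waits for an attribute, presumably mana, to cross a threshold.
; When triggered, it gets the units on the owner's team from the game state, applies GE_ValorBase to each, then clears the owner's mana.
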(event Ability|EventActivateAbility
  (Ability|ApplyGameplayEffectToOwner "/Game/Blueprints/Units/Chess/GE/NFC/Ge_PeriodicMana.Ge_PeriodicMana_C" 1 50)
  (Ability|Tasks|WaitForAttributeChangeThreshold "(AttributeName=\"Mana\",Attribute=/Script/AutoChess.AutoChessAttributeSet:Mana,AttributeOwner=\"/Script/CoreUObject.Class'/Script/AutoChess.AutoChessAttributeSet'\")" "GreaterThanOrEqualTo" 1e+02 false 0
    (:OnChange
      (bind _teamunits (Class|BPICore|GetUnits(Message) (Game|GetGameState) (Variables|/Script/AutoChess.AutoChessUnitBase|GetTeamID (.AsAutoChessUnitBase (CallFunction|GetAbilityOwnerActor self)))))
      (for _array_element _teamunits
        (GameplayEffects|ApplyGameplayEffectToTarget (Ability|TargetData|AbilityTargetDatafromActor _array_element) "/Game/Blueprints/Units/Chess/GE/GE_ValorBase.GE_ValorBase_C" 1 2))
      (Ability|ApplyGameplayEffectToOwner "/Game/Blueprints/Units/Chess/GE/NFC/Ge_ClearMana.Ge_ClearMana_C"))))