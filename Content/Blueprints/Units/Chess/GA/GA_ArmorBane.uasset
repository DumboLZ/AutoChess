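; GA_ArmorBane is a gameplay ability that applies armor-bane damage when an auto-chess attack hits an armored target.
; On activation it waits for the AutoChess.Event.Attack gameplay event and reads the target and attacker from the payload.
; If the target's armor attribute is above zero and the payload instigator's Instigator has the Empowered.ArmorBane state tag, it applies GE_ArmorBaneDamage to that target.
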(event Ability|EventActivateAbility
  (bind _payload (Ability|Tasks|WaitGameplayEvent "(TagName=\"AutoChess.Event.Attack\")" 0) ; 监听攻击事件
    (:EventReceived
      (if (Math|Boolean|ANDBoolean (.bSuccessfullyFoundAttribute (Ability|Attribute|GetFloatAttributefromAbilitySystemComponent (Ability|GetAbilitySystemComponent (.target _payload)) "(AttributeName=\"Shield\",Attribute=/Script/AutoChess.AutoChessAttributeSet:Shield,AttributeOwner=\"/Script/CoreUObject.Class'/Script/AutoChess.AutoChessAttributeSet'\")")) (> (.ReturnValue (Ability|Attribute|GetFloatAttributefromAbilitySystemComponent (Ability|GetAbilitySystemComponent (.target _payload)) "(AttributeName=\"Shield\",Attribute=/Script/AutoChess.AutoChessAttributeSet:Shield,AttributeOwner=\"/Script/CoreUObject.Class'/Script/AutoChess.AutoChessAttributeSet'\")")) 0.0) (GameplayTags|HasMatchingGameplayTag (Ability|GetAbilitySystemComponent (Variables|/Script/Engine.Actor|GetInstigator (.instigator _payload))) "(TagName=\"AutoChess.State.Empowered.ArmorBane\")"))
        (GameplayEffects|ApplyGameplayEffectToTarget (Ability|TargetData|AbilityTargetDatafromActor (.target _payload)) "/Game/Blueprints/Units/Chess/GE/GE_ArmorBaneDamage.GE_ArmorBaneDamage_C" 1 1)))))