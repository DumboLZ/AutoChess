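; GA_GMC03 is an auto-chess unit gameplay ability that stuns enemies around the caster.
; On activation it gets the 3x3 grid around the owner's current position and looks up each cell's unit through the game state.
; Units on another team receive GE_Stunned with two stacks, although the inline comment describes a 40 HP loss.
; The graph has no validity check on looked-up units and never calls EndAbility.
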(event Ability|EventActivateAbility
  (bind _asauto_chess_unit_base (Utilities|Casting|CastToAutoChessUnitBase (Components|GetOwner (Ability|GetAbilitySystemComponentfromActorInfo))))
  (bind _outputpoints (CallFunction|GetGrid3*3 (Variables|/Script/AutoChess.AutoChessUnitBase|GetCurrentGridPos _asauto_chess_unit_base)))
  (for _array_element _outputpoints
    (bind _asauto_chess_game_state (Utilities|Casting|CastToAutoChessGameState (Game|GetGameState)))
    (bind _returnvalue (Class|AutoChessGameState|GetUnitatGrid _asauto_chess_game_state (.X (Utilities|Struct|BreakIntPoint _array_element)) (.Y (Utilities|Struct|BreakIntPoint _array_element))))
    (if (not (== (Variables|/Script/AutoChess.AutoChessUnitBase|GetTeamID _returnvalue) (Variables|/Script/AutoChess.AutoChessUnitBase|GetTeamID (.AsAuto%20Chess%20Unit%20Base (Utilities|Casting|CastToAutoChessUnitBase (Ability|GetAvatarActorfromActorInfo)))))) ; 对敌人释放
      (GameplayEffects|ApplyGameplayEffectToTarget (Ability|TargetData|AbilityTargetDatafromActor _returnvalue) "/Game/Blueprints/Units/Chess/GE/GE_Stunned.GE_Stunned_C" 1 2) ; 流失40HP
    )))

(event Ability|EventOnEndAbility
  (params (bWasCancelled :type Boolean)))