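; GA_Javellin is a chess unit Gameplay Ability that listens for attack events and acts on Javellin-empowered attackers.
; On such attacks it applies GE_ArmorBaneDamage and GE_JavellinStack with negative stacks, the latter aimed at the attack target, then removes ArmorBane-tagged effects from the attacker.
; It then checks the attacker's GE_ArmorBaneDamage count, debug-printing it if positive, otherwise removing the Javellin empowered effect.
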(event Ability|EventActivateAbility
  (bind _payload (Ability|Tasks|WaitGameplayEvent "(TagName=\"AutoChess.Event.Attack\")" 0) ; 监听攻击事件
    (:EventReceived
      (Utilities|FlowControl|Sequence
        (:then_1
          (if (GameplayTags|HasMatchingGameplayTag (Ability|GetAbilitySystemComponent (Variables|/Script/Engine.Actor|GetInstigator (.instigator _payload))) "(TagName=\"AutoChess.State.Empowered.Javellin\")")
            (GameplayEffects|ApplyGameplayEffectToTarget :GameplayEffectClass "/Game/Blueprints/Units/Chess/GE/GE_ArmorBaneDamage.GE_ArmorBaneDamage_C" :Stacks -1)
            (GameplayEffects|ApplyGameplayEffectToTarget (Ability|TargetData|AbilityTargetDatafromActor (.target _payload)) "/Game/Blueprints/Units/Chess/GE/GE_JavellinStack.GE_JavellinStack_C" 1 -1)
            (GameplayEffects|RemoveActiveEffectswithTags (Ability|GetAbilitySystemComponent (Variables|/Script/Engine.Actor|GetInstigator (.instigator _payload))) "(GameplayTags=((TagName=\"AutoChess.State.Empowered.ArmorBane\")))")))
        (:then_2
          (if (> (GameplayEffects|GetGameplayEffectCount (Ability|GetAbilitySystemComponent (Variables|/Script/Engine.Actor|GetInstigator (.instigator _payload))) "/Game/Blueprints/Units/Chess/GE/GE_ArmorBaneDamage.GE_ArmorBaneDamage_C" 0 true) 0)
            (Development|PrintString (Utilities|String|ToString(Integer) (GameplayEffects|GetGameplayEffectCount (Ability|GetAbilitySystemComponent (Variables|/Script/Engine.Actor|GetInstigator (.instigator _payload))) "/Game/Blueprints/Units/Chess/GE/GE_ArmorBaneDamage.GE_ArmorBaneDamage_C" 0 true)))
            (else
              (GameplayEffects|RemoveActiveEffectswithTags (Ability|GetAbilitySystemComponent (Variables|/Script/Engine.Actor|GetInstigator (.instigator _payload))) "(GameplayTags=((TagName=\"AutoChess.State.Empowered.Javellin\")))"))))))))