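; GA_AUC01 is an auto-chess unit Gameplay Ability that trades HP for armor on units in the 3x3 grid around its owner.
; On activation it gets those cells from the owner's grid position, draws debug spheres and looks up each cell's unit through AutoChessGameState.
; Each unit receives stacked HP-loss and shield Gameplay Effects, with no team filter.
; The graph never calls EndAbility.
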(event Ability|EventActivateAbility
  (bind _asauto_chess_unit_base (Utilities|Casting|CastToAutoChessUnitBase (Components|GetOwner (Ability|GetAbilitySystemComponentfromActorInfo))))
  (bind _outputpoints (CallFunction|GetGrid3*3 (Variables|/Script/AutoChess.AutoChessUnitBase|GetCurrentGridPos _asauto_chess_unit_base)))
  (for _array_element _outputpoints
    (Rendering|Debug|DrawDebugSphere (Math|Vector|MakeVectorNetQuantize (Math|Conversions|ToFloat(Integer) (+ (* (.X (Utilities|Struct|BreakIntPoint _array_element)) 100) 50)) (Math|Conversions|ToFloat(Integer) (+ (* (.Y (Utilities|Struct|BreakIntPoint _array_element)) 100) 50)) 108.0) 5e+01 12 "(R=1.000000,G=1.000000,B=1.000000,A=1.000000)" 5.0)
    (bind _asauto_chess_game_state (Utilities|Casting|CastToAutoChessGameState (Game|GetGameState)))
    (bind _returnvalue (Class|AutoChessGameState|GetUnitatGrid _asauto_chess_game_state (.X (Utilities|Struct|BreakIntPoint _array_element)) (.Y (Utilities|Struct|BreakIntPoint _array_element))))
    (GameplayEffects|ApplyGameplayEffectToTarget (Ability|TargetData|AbilityTargetDatafromActor _returnvalue) "/Game/Blueprints/Units/Chess/GE/GE_HPLoss.GE_HPLoss_C" 1 40) ; 流失40HP
    (GameplayEffects|ApplyGameplayEffectToTarget (Ability|TargetData|AbilityTargetDatafromActor _returnvalue) "/Game/Blueprints/Units/Card/GE/GE_Shield25.GE_Shield25_C" 1 4) ; 获得100护甲
  ))

(event Ability|EventOnEndAbility
  (params (bWasCancelled :type Boolean)))