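; GA_GRC03 is a gameplay ability for an auto-chess unit that weakens every enemy unit's maximum health.
; On activation it gets the avatar unit's team, fetches all units of the opposing team from the auto-chess game state, and applies GE_ReduceMaxHP to each one.
; The opposing team is derived by flipping a two-team ID, and the ability never calls EndAbility.
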(event Ability|EventActivateAbility
  (bind _asbp_auto_chess_game_state (Utilities|Casting|CastToBP_AutoChessGameState (Game|GetGameState)))
  (bind _asauto_chess_unit_base (Utilities|Casting|CastToAutoChessUnitBase (Ability|GetAvatarActorfromActorInfo)))
  (bind _returnvalue (Class|AutoChessGameState|GetUnitsbyTeam _asbp_auto_chess_game_state (Math|Integer|Absolute(Integer) (- 1 (Variables|/Script/AutoChess.AutoChessUnitBase|GetTeamID _asauto_chess_unit_base)))))
  (for _array_element _returnvalue
    (GameplayEffects|ApplyGameplayEffectToTarget (Ability|TargetData|AbilityTargetDatafromActor _array_element) "/Game/Blueprints/Units/Chess/GE/GE_ReduceMaxHP.GE_ReduceMaxHP_C" 1 1)))